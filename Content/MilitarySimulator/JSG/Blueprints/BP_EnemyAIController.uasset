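; AI controller for enemies that turns sight and hearing perception into Blackboard data on the server.
; Seeing an actor sets TargetActor and, if bCanFocusOn, focuses it.
; Losing sight saves the target's position to the Blackboard and a placed BP_LastKnownLocationActor, then clears target and focus.
; Heard sounds write their location to TargetLocation; debug prints show perception changes and the current target each tick.
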(event OnTargetPerceptionUpdated(AIPerception)
  (params (Actor :type Actor%20Object%20Reference) (Stimulus :type AI%20Stimulus%20Structure))
  (bind (_age _expirationage _strength _stimuluslocation _receiverlocation _tag _bsuccessfullysensed) (Utilities|Struct|BreakAIStimulus Stimulus))
  (bind _returnvalue (Utilities|Name|MakeLiteralName "TargetActor"))
  (bind _lastknownlocationactor (Variables|Default|GetLastKnownLocationActor))
  (bind _blackboard (Variables|Default|GetBlackboard))
  (if (Ability|HasAuthority (Pawn|GetControlledPawn))
    ;[0.5139 1 0.3498] AISense_Sight (에너미 시각) Update
    (Variables|Default|SetSensedActor Actor)
    (bind _returnvalue_2 (Class|AIPerceptionSystem|GetSenseClassforStimulus Stimulus))
    (if (== _returnvalue_2 "/Script/AIModule.AISense_Sight")
      (if _bsuccessfullysensed
        (AI|Components|Blackboard|SetValueasObject _blackboard _returnvalue (Variables|Default|GetSensedActor))
        (if (ScalableFloat|GetValueasBool (Variables|Default|GetBlackboard) (Utilities|Name|MakeLiteralName "bCanFocusOn"))
          (AI|SetFocus (Variables|Default|GetSensedActor))
          (Development|PrintString "AISense_Sigth [Detect] The Player"))
        (else
          (bind _asactor (Utilities|Casting|CastToActor (AI|Components|Blackboard|GetValueasObject _blackboard _returnvalue)))
          (AI|Components|Blackboard|SetValueasVector _blackboard (Utilities|Name|MakeLiteralName "LaskKnownLocation") (Transformation|GetActorLocation _asactor))
          (Transformation|SetActorLocation _lastknownlocationactor (Transformation|GetActorLocation _asactor) false true)
          (Development|PrintString (Utilities|String|ToString(Vector) (Transformation|GetActorLocation _lastknownlocationactor)) true false "(R=1.000000,G=0.831519,B=0.000000,A=1.000000)" 1e+01)
          (AI|Components|Blackboard|ClearValue _blackboard (Utilities|Name|MakeLiteralName "TargetActor"))
          (AI|ClearFocus)
          (Development|PrintString "AISense_Sigth [Lost] The Player")))
      (else
        (Development|PrintString "This Sense is not Sight")
        ;[0.4703 0.709 1] AISense_Hearing(에너미 청각) Update
        (if (== _returnvalue_2 "/Script/AIModule.AISense_Hearing")
          (AI|Components|Blackboard|SetValueasVector (Variables|Default|GetBlackboard) (Utilities|Name|MakeLiteralName "TargetLocation") _stimuluslocation)
          (Development|PrintString "AISense_Hearing [Heard] Player's Sound"))))))

(event EventBeginPlay
  (bind _returnvalue (Actor|GetActorOfClass "/Game/MilitarySimulator/JSG/EnemyAI/Contexts/BP_LastKnownLocationActor.BP_LastKnownLocationActor_C"))
  (Utilities|IsValid _returnvalue
    (:Is%20Valid
      (Variables|Default|SetLastKnownLocationActor _returnvalue))
    (:Is%20Not%20Valid
      (Development|PrintString "BP_LaskKnownLocationActor is not exist"))))

(event EventTick
  (params (DeltaSeconds :type Float%20%28single-precision%29))
  (CallFunction|NewFunction DeltaSeconds))

(fn ConstructionScript)

(fn NewFunction
  (params (DeltaSeconds :type Float%20%28double-precision%29))
  (bind _asactor (Utilities|Casting|CastToActor (AI|Components|Blackboard|GetValueasObject (Variables|Default|GetBlackboard) (Utilities|Name|MakeLiteralName "TargetActor")))
    (:then
      (Development|PrintString (Utilities|String|ToString(Text) (Utilities|Text|FormatText "TargetActor: {TA}" _asactor)) true false "(R=0.000000,G=0.660000,B=1.000000,A=1.000000)" DeltaSeconds))
    (:CastFailed
      (Development|PrintString "TargetActor is not valid" true false "(R=0.000000,G=0.660000,B=1.000000,A=1.000000)" DeltaSeconds))))