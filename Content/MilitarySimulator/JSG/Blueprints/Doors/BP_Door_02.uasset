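; BP_Door_02 is a networked door actor that players in range toggle open and closed.
; Its trigger overlap enables input and makes the character the owner, allowing the input action to call a server RPC, and clears both on exit.
; The server multicasts the toggle, which plays a 2D sound and runs a timeline forward or backward to drive the door's yaw, with a Moving flag blocking input mid-swing.
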(event OnComponentBeginOverlap(Trigger)
  (params (OverlappedComponent :type Primitive%20Component%20Object%20Reference) (OtherActor :type Actor%20Object%20Reference) (OtherComp :type Primitive%20Component%20Object%20Reference) (OtherBodyIndex :type Integer) (bFromSweep :type Boolean) (SweepResult :type Hit%20Result%20Structure%20%28by%20ref%29))
  (bind _ascharacter (Utilities|Casting|CastToCharacter OtherActor))
  (bind _asplayer_controller (Utilities|Casting|CastToPlayerController (Pawn|GetController _ascharacter)))
  (Input|EnableInput _asplayer_controller)
  (Actor|SetOwner OtherActor)
  (Development|PrintString "In Door Range"))

(event OnComponentEndOverlap(Trigger)
  (params (OverlappedComponent :type Primitive%20Component%20Object%20Reference) (OtherActor :type Actor%20Object%20Reference) (OtherComp :type Primitive%20Component%20Object%20Reference) (OtherBodyIndex :type Integer))
  (bind _ascharacter (Utilities|Casting|CastToCharacter OtherActor))
  (bind _asplayer_controller (Utilities|Casting|CastToPlayerController (Pawn|GetController _ascharacter)))
  (Input|DisableInput _asplayer_controller)
  (Actor|SetOwner 0)
  (Development|PrintString "Exit Door Range"))

(event Custom|MulticastRPC_RotateDoor
  (Variables|Default|SetbMoving true)
  (bind _output_get (Variables|Default|SetbIsOpen (not (Variables|Default|GetbIsOpen))))
  (if _output_get
    (Audio|SpawnSound2D "/Game/BrickBuilding/Sounds/A_Open_Door_01_Cue.A_Open_Door_01_Cue" 1.0 1.0 0.0 0)
    (bind (_direction _newtrack_0) (Timeline|Timeline Play)
      (:Update
        (Transformation|SetRelativeRotation (Variables|Default|GetDoor01) (Math|Rotator|MakeRotator 0.0 0.0 _newtrack_0) false false))
      (:Finished
        (Variables|Default|SetbMoving false)))
    (else
      (Audio|SpawnSound2D "/Game/BrickBuilding/Sounds/A_Closing_Door_01_Cue.A_Closing_Door_01_Cue" 1.0 1.0 0.0 0)
      (Timeline|Timeline Reverse))))

(event Custom|ServerRPC_RotateDoor
  (CallFunction|MulticastRPCRotateDoor))

(event Input|EnhancedActionEvents|EnhancedInputActionIA_Door_Open
  (params (ActionValue :type Boolean) (ElapsedSeconds :type Float%20%28double-precision%29) (TriggeredSeconds :type Float%20%28double-precision%29) (InputAction :type Input%20Action%20Object%20Reference :default "/Game/MilitarySimulator/HSB/Input/Actions/IA_Door_Open.IA_Door_Open"))
  (:Started
    (if (not (Variables|Default|GetbMoving))
      (CallFunction|ServerRPCRotateDoor))))

(event EventBeginPlay)

(event Collision|EventActorBeginOverlap
  (params (OtherActor :type Actor%20Object%20Reference)))

(event EventTick
  (params (DeltaSeconds :type Float%20%28single-precision%29)))

(fn ConstructionScript)