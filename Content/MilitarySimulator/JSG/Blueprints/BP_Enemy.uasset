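; BP_Enemy is an AI enemy Blueprint whose only active graph logic is an on-screen debug readout of its state.
; Tick calls PrintState, which runs only with authority and shows the blackboard's LastKnownLocation and the enemy's current HP.
; Each message lasts one frame's DeltaSeconds, so the readout refreshes continuously without writing to the log.
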(event EventBeginPlay)

(event Collision|EventActorBeginOverlap
  (params (OtherActor :type Actor%20Object%20Reference)))

(event EventTick
  (params (DeltaSeconds :type Float%20%28single-precision%29))
  (CallFunction|PrintState DeltaSeconds))

(fn ConstructionScript)

(fn PrintState
  (params (DeltaSeconds :type Float%20%28double-precision%29))
  (Networking|SwitchHasAuthority
    (:Authority
      (Development|PrintText (Utilities|Text|FormatText "LaskKnownLocation: {location}" (Utilities|String|ToString(Vector) (AI|Components|Blackboard|GetValueasVector (AI|GetBlackboard 0) (Utilities|Name|MakeLiteralName "LastKnownLocation")))) true false "(R=1.000000,G=0.617207,B=0.309469,A=1.000000)" DeltaSeconds)
      (bind _returnvalue (Class|SGEnemy|GetHP))
      (Development|PrintString (Utilities|String|ToString(Text) (Utilities|Text|FormatText "EnemyHP: {hp}" _returnvalue)) true false "(R=1.000000,G=0.003031,B=0.000000,A=1.000000)" DeltaSeconds))))