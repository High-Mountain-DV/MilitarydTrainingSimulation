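; VR player gun with hand grabbing, trigger firing, magazine loading and a pullable charging handle.
; Grabbing attaches the gun to the hand and swaps per-hand input; magazine overlap copies ammo and attaches via RPCs.
; Timers drive the handle, whose full pull and release enables firing.
; Server RPC spawns bullets and AI noise, multicasting effects; mode switching and magazine dropping are stubs.
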(event OnComponentBeginOverlap(MagazineAttatchCollision)
  (params (OverlappedComponent :type Primitive%20Component%20Object%20Reference) (OtherActor :type Actor%20Object%20Reference) (OtherComp :type Primitive%20Component%20Object%20Reference) (OtherBodyIndex :type Integer) (bFromSweep :type Boolean) (SweepResult :type Hit%20Result%20Structure%20%28by%20ref%29))
  (Networking|SwitchHasAuthority
    (:Remote
      (bind _asbp_magazine (Utilities|Casting|CastToBP_Magazine OtherActor))
      (Utilities|FlowControl|DoOnce false
        (:Completed
          ;[1 1 1] Bullet 수 설정
          (Variables|Default|SetAmmoGun (Variables|/Game/MilitarySimulator/HSB/Blueprints/GunBlueprints/BP_Magazine.BP_Magazine_C|GetAmmo _asbp_magazine))
          (Default|Detach _asbp_magazine)
          (CallFunction|ServerRPCAttach _asbp_magazine))))))

(event Custom|ServerRPC_Attach
  (params (Mag :type BP%20Magazine%20Object%20Reference))
  (CallFunction|MultiRPCAttach Mag))

(event Custom|MultiRPC_Attach
  (params (Mag :type BP%20Magazine%20Object%20Reference))
  (bind _gunmesh (Variables|Default|GetGunMesh))
  (bind _returnvalue (Transformation|GetWorldTransform _gunmesh))
  (Transformation|SetActorTransform Mag (Math|Transform|MakeTransform (+ (.location _returnvalue) (* (Transformation|GetActorRightVector) 9.0)) (.rotation _returnvalue) (.scale _returnvalue)) false true)
  (Transformation|AttachComponentToComponent Mag (Variables|Default|GetGunMesh) "Magazine" "KeepWorld" "SnapToTarget" "KeepWorld" true)
  (Utilities|FlowControl|DoOnce false) ; enters at Reset
)

(event EventBeginPlay
  (bind _has_at_least_one_firing_mode (CallFunction|HasFiringModes))
  (if _has_at_least_one_firing_mode
    _))

(event OnGrabbed(GrabComponentSnap)
  (params (Motion%20Controller :type Motion%20Controller%20Component%20Object%20Reference))
  ;[0.03434 0.03434 0.03434] Main Grab
  (Variables|Default|SetGunGrab true)
  (|RemoveMappingContextfromOppositeHand&CleartheReference)
  (CallFunction|MappingContextGun)
  (bind _holding_hand_anim (CallFunction|GetHoldingHandAnim))
  (Variables|Default|SetHolding%20Hand%20Anim _holding_hand_anim)
  (CallFunction|ServerRPConGrabbed(GrabCompSnap) Motion%20Controller))

(event OnDropped(GrabComponentSnap)
  (CallFunction|ServerRPConDropped(GrabCompSnap)))

(event Custom|ServerRPC_OnGrabbed%28GrabCompSnap%29
  (params (Motion%20Controller :type Motion%20Controller%20Component%20Object%20Reference))
  ;[0.03434 0.03434 0.03434] Main Grab
  (bind _aspawn (Utilities|Casting|CastToPawn (Components|GetOwner Motion%20Controller)))
  (Variables|Actor|SetInstigator _aspawn)
  (bind _output_get (Variables|Default|SetMotion%20Controller Motion%20Controller))
  (Utilities|IsValid _output_get
    (:Is%20Valid
      (|AttachMainGripHandMeshToTheGun _output_get))))

(event Custom|ServerRPC_OnDropped%28GrabCompSnap%29
  (CallFunction|MultiRPConDropped(GrabCompSnap)))

(event Custom|MultiRPC_OnDropped%28GrabCompSnap%29
  (Variables|Default|SetGunGrab false))

(event Custom|Align%20Gun%20To%20Initial%20Position%20After%20Done%20Shooting
  (if true
    _))

(event Custom|ServerRPC_Fire
  (bind _instigator (Variables|Actor|GetInstigator))
  (CallFunction|MulticastRPCSpawnFireVFX)
  (bind _returnvalue (Game|SpawnActorfromClass "/Game/MilitarySimulator/JSG/Blueprints/BP_EnemyBullet.BP_EnemyBullet_C" (Transformation|GetWorldTransform (Variables|Default|GetFirePosition)) "AlwaysSpawn" "MultiplyWithRoot" _instigator _instigator))
  (Class|AISenseHearing|ReportNoiseEvent (Transformation|GetWorldLocation (Variables|Default|GetFirePosition)) 1e+01 (Variables|Actor|GetInstigator) 1e+04 "None")
  (Utilities|PrintBulletState _returnvalue))

(event Custom|MulticastRPC_SpawnFireVFX
  (bind _fireposition (Variables|Default|GetFirePosition))
  (bind _returnvalue (Transformation|GetWorldLocation _fireposition))
  (Effects|SpawnEmitteratLocation "/Game/StarterContent/Particles/P_Explosion.P_Explosion" _returnvalue "0, 0, 0" "0.200000,0.200000,0.200000")
  (Audio|PlaySoundatLocation "/Game/MilitarySimulator/HSB/Assets/Sound/Rifle.Rifle" _returnvalue "0, 0, 0" 1.0 1.0 0.0 0 0 0 0))

(event Input|EnhancedActionEvents|EnhancedInputActionIA_GunShoot_Left
  (params (ActionValue :type Float%20%28double-precision%29) (ElapsedSeconds :type Float%20%28double-precision%29) (TriggeredSeconds :type Float%20%28double-precision%29) (InputAction :type Input%20Action%20Object%20Reference :default "/Game/MilitarySimulator/HSB/Input/Actions/IA_GunShoot_Left.IA_GunShoot_Left"))
  (:Started
    (|LeftHandFireTrigger ActionValue :!label _label
      (:Trigger%20Passed%20Threshold
        ;[1 1 1] 총-shooting
        (Utilities|FlowControl|Sequence
          (:then_0
            (if (Math|Boolean|ANDBoolean (Variables|Default|GetGunGrab) (Variables|Default|GetSliderReleased) (> (Variables|Default|GetAmmoGun) 0))
              (CallFunction|ServerRPCFire)
              (Math|Integer|DecrementInt (Variables|Default|GetAmmoGun))))))
      (:Trigger%20Has%20Not%20Passed%20Threshold
        (Utilities|FlowControl|DoOnce false
          (:Completed
            (CallFunction|AlignGuntoInitialPositionAfterDoneShooting))))))
  (:Canceled
    (goto _label Trigger%20Is%20Not%20Pressed%20/%20Canceled))
  (:Completed
    (goto _label Trigger%20Is%20Not%20Pressed%20/%20Canceled)))

(event Input|EnhancedActionEvents|EnhancedInputActionIA_GunShoot_Right
  (params (ActionValue :type Float%20%28double-precision%29) (ElapsedSeconds :type Float%20%28double-precision%29) (TriggeredSeconds :type Float%20%28double-precision%29) (InputAction :type Input%20Action%20Object%20Reference :default "/Game/MilitarySimulator/HSB/Input/Actions/IA_GunShoot_Right.IA_GunShoot_Right"))
  (:Started
    (|RightHandFireTrigger ActionValue :!label _label
      (:Trigger%20Passed%20Threshold
        ;[1 1 1] 총-shooting
        (Utilities|FlowControl|Sequence
          (:then_0
            (if (Math|Boolean|ANDBoolean (Variables|Default|GetGunGrab) (Variables|Default|GetSliderReleased) (> (Variables|Default|GetAmmoGun) 0))
              (CallFunction|ServerRPCFire)
              (Math|Integer|DecrementInt (Variables|Default|GetAmmoGun))))))
      (:Trigger%20Has%20Not%20Passed%20Threshold
        (Utilities|FlowControl|DoOnce false
          (:Completed
            (CallFunction|AlignGuntoInitialPositionAfterDoneShooting))))))
  (:Canceled
    (goto _label Trigger%20Is%20Not%20Pressed%20/%20Canceled))
  (:Completed
    (goto _label Trigger%20Is%20Not%20Pressed%20/%20Canceled)))

(event OnGrabbed(CurlGrabComponentSlide)
  (params (Motion%20Controller :type Motion%20Controller%20Component%20Object%20Reference))
  ;[0 0 0] Grabbing Slider
  (CallFunction|AttachHandtoSlide Motion%20Controller)
  (Audio|PlaySoundatLocation "/Game/MilitarySimulator/HSB/Assets/Sound/Reload.Reload" (Transformation|GetWorldLocation (Variables|Default|GetSliderGrabCollision)) "0, 0, 0" 2.0 1.0 0.0 0 0 0 0)
  (Variables|Default|SetInitial%20Grab%20Offset (CallFunction|GetGrabOffsetBetweenMC&Slide))
  (Variables|Default|SetSliderReleased false)
  (Utilities|Time|SetTimerbyEvent (delegate Custom|Interpolate%20Slide%20Movement) 0.01 true))

(event OnDropped(CurlGrabComponentSlide)
  ;[0 0 0] Releasing the Handle
  (CallFunction|DetachHandfromSlide)
  (Variables|Default|SetSlideGrabMotionController 0)
  (Variables|Default|SetSlideMotionControllerHandMesh 0)
  (Class|KismetSystemLibrary|PauseTimer 0 "Interpolate Slide Movement")
  (if (<= (Variables|Default|GetCurrent%20Slide%20Offset) (Variables|Default|GetChargingHandleMaxDistance))
    (Variables|Default|SetSliderReleased true))
  (Utilities|Time|SetTimerbyEvent (delegate Custom|Return%20Slider%20Back) 0.01 true)
  ;;[1 1 1] Play Release Sound
  (Audio|PlaySoundatLocation (Variables|Default|GetSlideReleasedSoundCue) (Transformation|GetWorldLocation (Variables|Default|GetMuzzle)) "0, 0, 0" 1.0 1.0 0.0 0 0 0 0))

(event Custom|Interpolate%20Slide%20Movement
  ;[0 0 0] Grabbing Slider
  (bind _returnvalue (CallFunction|ClampSlideMovement (Variables|Default|GetChargingHandleMaxDistance)))
  (Variables|Default|SetCurrent%20Slide%20Offset _returnvalue)
  (Development|PrintString (Utilities|String|ToString(Text) (Utilities|Text|FormatText "CurrentSlideOffset: {0}" (Variables|Default|GetCurrent%20Slide%20Offset))))
  (if (and (<= _returnvalue (Variables|Default|GetChargingHandleMaxDistance)) (not (Variables|Default|GetReachedLockPosition)))
    ;;[1 1 1] Play Slide Cocked Sound
    (Variables|Default|SetReachedLockPosition true)
    (Development|PrintString "ReachedLockPosition!")
    (Audio|PlaySoundatLocation (Variables|Default|GetCockedSoundCue) (Transformation|GetWorldLocation (Variables|Default|GetSliderGrabCollision)) "0, 0, 0" 1.0 1.0 0.0 0 0 0 0))
  (Transformation|SetRelativeLocation (Variables|Default|GetHandle) (Math|Vector|MakeVector 0.0 (Variables|Default|GetCurrent%20Slide%20Offset) 0.0) false false))

(event Custom|Return%20Slider%20Back
  ;[0 0 0] Releasing the Handle
  (bind _has_reached_origin (CallFunction|InterpolateHandletoInitialPositionandContinueOnceDone))
  (if _has_reached_origin
    (Transformation|SetRelativeLocation (Variables|Default|GetHandle) (Math|Vector|MakeVector 0.0 0.0 0.0) false false)
    (Class|KismetSystemLibrary|PauseTimer 0 "Return Slider Back")
    (Variables|Default|SetCurrent%20Slide%20Offset 0.0)
    (if (Variables|Default|GetReachedLockPosition)
      ;;[0.3003 0.3003 0.3003] 총알 장전 로직 (그냥 slider 당기면 발사되는 걸로)
      (bind _magazine (Variables|Default|GetMagazine)
        (:then
          (if (Variables|Default|GetBullet%20Is%20Ready%20to%20be%20Taken%20from%20Mag)
            (if (Variables|/Game/MilitarySimulator/HSB/Blueprints/GunBlueprints/BP_Magazine.BP_Magazine_C|GetIs%20Empty _magazine)
              (if (Variables|Default|GetChamber%20Has%20Bullet)
                (Variables|Default|SetDry%20Fire true :!label _label)
                (Rendering|SetVisibility (Variables|Default|GetRound) false false)
                (Variables|Default|SetChamber%20Has%20Bullet false))
              (else
                (Default|RemoveRound (Variables|Default|GetMagazine))
                (Rendering|SetVisibility (Variables|Default|GetRound) true false)
                (Variables|Default|SetChamber%20Has%20Bullet true)))
            (else
              (Variables|Default|SetReachedLockPosition false :!label _label_2)
              (goto _label))))
        (:else
          (goto _label_2))))))

(event OnComponentBeginOverlap(MagazineCollision)
  (params (OverlappedComponent :type Primitive%20Component%20Object%20Reference) (OtherActor :type Actor%20Object%20Reference) (OtherComp :type Primitive%20Component%20Object%20Reference) (OtherBodyIndex :type Integer) (bFromSweep :type Boolean) (SweepResult :type Hit%20Result%20Structure%20%28by%20ref%29)))

(event Custom|Simulate%20Magazine%20Physics%20On%20Dropped
  (params (Motion%20Controller :type Motion%20Controller%20Component%20Object%20Reference))
  (Variables|/Game/MilitarySimulator/HSB/Blueprints/GrabComponent.GrabComponent_C|SetbSimulateOnDrop (Variables|/Game/MilitarySimulator/HSB/Blueprints/GunBlueprints/BP_Magazine.BP_Magazine_C|GetGrabComponentSnap (Variables|Default|GetMagazine)) true)
  (EventDispatchers|UnbindEventfromOnGrabbed (Variables|/Game/MilitarySimulator/HSB/Blueprints/GunBlueprints/BP_Magazine.BP_Magazine_C|GetGrabComponentSnap (Variables|Default|GetMagazine)) (delegate Custom|Simulate%20Magazine%20Physics%20On%20Dropped))
  (Variables|Default|SetMagazine 0))

(event Custom|Smooth%20Attachment
  (bind _returnvalue (CallFunction|SmoothMagazineAttachmentandContinueOnceDone))
  (if _returnvalue
    (Transformation|AttachComponentToComponent (Variables|Default|GetMagazine) (Variables|Default|GetGunMesh) "Magazine" "SnapToTarget" "SnapToTarget" "SnapToTarget" true)
    (Class|KismetSystemLibrary|PauseTimer 0 "Smooth Attachment")))

(event Input|EnhancedActionEvents|EnhancedInputActionIA_DropMag_Left
  (params (ActionValue :type Boolean) (ElapsedSeconds :type Float%20%28double-precision%29) (TriggeredSeconds :type Float%20%28double-precision%29) (InputAction :type Input%20Action%20Object%20Reference :default "/Game/MilitarySimulator/HSB/Input/Actions/IA_DropMag_Left.IA_DropMag_Left")))

(event Input|EnhancedActionEvents|EnhancedInputActionIA_DropMag_Right
  (params (ActionValue :type Boolean) (ElapsedSeconds :type Float%20%28double-precision%29) (TriggeredSeconds :type Float%20%28double-precision%29) (InputAction :type Input%20Action%20Object%20Reference :default "/Game/MilitarySimulator/HSB/Input/Actions/IA_DropMag_Right.IA_DropMag_Right")))

(event Input|EnhancedActionEvents|EnhancedInputActionIA_SwitchGunMode_Left
  (params (ActionValue :type Boolean) (ElapsedSeconds :type Float%20%28double-precision%29) (TriggeredSeconds :type Float%20%28double-precision%29) (InputAction :type Input%20Action%20Object%20Reference :default "/Game/MilitarySimulator/HSB/Input/Actions/IA_SwitchGunMode_Left.IA_SwitchGunMode_Left"))
  (:Completed
    (CallFunction|SwitchGunMode)
    (CallFunction|RotateSelectorMesh)))

(event Input|EnhancedActionEvents|EnhancedInputActionIA_SwitchGunMode_Right
  (params (ActionValue :type Boolean) (ElapsedSeconds :type Float%20%28double-precision%29) (TriggeredSeconds :type Float%20%28double-precision%29) (InputAction :type Input%20Action%20Object%20Reference :default "/Game/MilitarySimulator/HSB/Input/Actions/IA_SwitchGunMode_Right.IA_SwitchGunMode_Right"))
  (:Completed
    (CallFunction|SwitchGunMode)
    (CallFunction|RotateSelectorMesh)))

(fn ConstructionScript)

(fn GetHoldingHandAnim
  (bind _grabcomponentsnap (Variables|Default|GetGrabComponentSnap))
  (if (Utilities|Enum|Equal(Enum) (Default|GetHeldbyHand _grabcomponentsnap) "Left")
    (return (Variables|/Game/MilitarySimulator/HSB/Blueprints/GrabComponent.GrabComponent_C|GetLeft%20Hand%20Anim _grabcomponentsnap))
    (else
      (return (Variables|/Game/MilitarySimulator/HSB/Blueprints/GrabComponent.GrabComponent_C|GetRight%20Hand%20Anim _grabcomponentsnap)))))

(fn AttachHandtoSlide
  (params (Motion%20Controller :type Motion%20Controller%20Component%20Object%20Reference))
  (bind _asbp_player_vr (Utilities|Casting|CastToBP_PlayerVR (Components|GetOwner)))
  (Transformation|AttachComponentToComponent (Variables|/Game/MilitarySimulator/HSB/Blueprints/BP_PlayerVR.BP_PlayerVR_C|GetSK_HandLeft _asbp_player_vr) (Variables|Default|GetSlideHand_L) "" "SnapToTarget" "SnapToTarget" "KeepRelative" true)
  (return))

(fn DetachHandfromSlide
  (bind _asbp_player_vr (Utilities|Casting|CastToBP_PlayerVR (Components|GetOwner)))
  (if (Utilities|Enum|Equal(Enum) (Default|GetHeldbyHand (Variables|Default|GetCurlGrabComponentSlide)) "Right")
    ;[1 1 1] Hand Right
    ;;[0 0 0] Hand를 다시 PlayerVR pawn에 붙임
    (Transformation|AttachComponentToComponent (Variables|/Game/MilitarySimulator/HSB/Blueprints/BP_PlayerVR.BP_PlayerVR_C|GetSK_HandRight _asbp_player_vr) (Variables|/Game/MilitarySimulator/HSB/Blueprints/BP_PlayerVR.BP_PlayerVR_C|GetMotionControllerRightGrip _asbp_player_vr) "None" "SnapToTarget" "SnapToTarget" "SnapToTarget" true)
    (Transformation|AddRelativeRotation (Variables|/Game/MilitarySimulator/HSB/Blueprints/BP_PlayerVR.BP_PlayerVR_C|GetSK_HandRight _asbp_player_vr) "-1.000000,-389.500000,-275.000000" false false)
    (else
      ;[1 1 1] Hand Left
      (Transformation|AttachComponentToComponent (Variables|/Game/MilitarySimulator/HSB/Blueprints/BP_PlayerVR.BP_PlayerVR_C|GetSK_HandLeft _asbp_player_vr) (Variables|/Game/MilitarySimulator/HSB/Blueprints/BP_PlayerVR.BP_PlayerVR_C|GetMotionControllerLeftGrip _asbp_player_vr) "None" "SnapToTarget" "SnapToTarget" "SnapToTarget" true)
      (Transformation|AddRelativeRotation (Variables|/Game/MilitarySimulator/HSB/Blueprints/BP_PlayerVR.BP_PlayerVR_C|GetSK_HandLeft _asbp_player_vr) "1.000000,-150.500000,85.000000" false false)))
  (Transformation|SetRelativeLocation (Variables|/Game/MilitarySimulator/HSB/Blueprints/BP_PlayerVR.BP_PlayerVR_C|GetSK_HandRight _asbp_player_vr) "0.000000,0.000000,4.000000" false false)
  (Transformation|AttachComponentToComponent (Variables|Default|GetSliderGrabCollision) (Variables|Default|GetSliderPosition) "None" "SnapToTarget" "SnapToTarget" "SnapToTarget" true)
  (return))

(fn GetGrabOffsetBetweenMC&Slide
  (return (- (Transformation|GetWorldLocation (Variables|/Game/MilitarySimulator/HSB/Blueprints/CurlGrabComponent.CurlGrabComponent_C|GetMotionControllerRef (Variables|Default|GetCurlGrabComponentSlide))) (Transformation|GetWorldLocation (Variables|Default|GetHandle)))))

(fn ClampSlideMovement
  (params (Min :type Float%20%28double-precision%29))
  (return (Math|Float|Clamp(Float) (+ (.y (Math|Transform|InverseTransformLocation (Transformation|GetWorldTransform (Variables|Default|GetHandle)) (- (Transformation|GetWorldLocation (Variables|/Game/MilitarySimulator/HSB/Blueprints/CurlGrabComponent.CurlGrabComponent_C|GetMotionControllerRef (Variables|Default|GetCurlGrabComponentSlide))) (Variables|Default|GetInitial%20Grab%20Offset)))) (.y (Variables|/Script/Engine.SceneComponent|GetRelativeLocation (Variables|Default|GetHandle)))) Min 0.0)))

(fn InterpolateHandletoInitialPositionandContinueOnceDone
  (bind _returnvalue (Utilities|Time|GetWorldDeltaSeconds))
  (bind _handle (Variables|Default|GetHandle))
  (bind _slidersnaptooriginspeedmultiplier (Variables|Default|GetSliderSnapToOriginSpeedMultiplier))
  (bind _returnvalue_2 (* _returnvalue _slidersnaptooriginspeedmultiplier))
  (bind _relativelocation (Variables|/Script/Engine.SceneComponent|GetRelativeLocation _handle))
  (bind _returnvalue_3 (Math|Interpolation|FInterpTo (.y _relativelocation) 0.0 _returnvalue_2 0.4))
  (Transformation|SetRelativeLocation _handle (Math|Vector|MakeVector 0.0 _returnvalue_3 0.0) false false)
  (return (Math|Float|NearlyEqual(Float) _returnvalue_3 0.0 0.01)))

(fn HasFiringModes
  (return (> (Utilities|Array|Length (Variables|Default|GetFiring%20Modes)) 0)))

(fn SwitchGunMode)

(fn RotateSelectorMesh)

(fn StoreGunLocation&Rotation
  (bind _gunmesh (Variables|Default|GetGunMesh))
  (Variables|Default|SetRelative%20Location (Variables|/Script/Engine.SceneComponent|GetRelativeLocation _gunmesh))
  (Variables|Default|SetRelative%20Rotation (Variables|/Script/Engine.SceneComponent|GetRelativeRotation _gunmesh))
  (return))

(fn SmoothMagazineAttachmentandContinueOnceDone
  (bind _returnvalue (Utilities|Time|GetWorldDeltaSeconds))
  (bind _magazine (Variables|Default|GetMagazine))
  (bind _gunmesh (Variables|Default|GetGunMesh))
  (bind _magazinesnapspeedmultiplier (Variables|Default|GetMagazineSnapSpeedMultiplier))
  (bind _returnvalue_2 (Transformation|GetSocketLocation _gunmesh "Magazine"))
  (bind _returnvalue_3 (* _returnvalue _magazinesnapspeedmultiplier))
  (bind _grippable_magazine_mesh (Variables|/Game/MilitarySimulator/HSB/Blueprints/GunBlueprints/BP_Magazine.BP_Magazine_C|GetGrippable%20Magazine%20Mesh _magazine))
  (bind _returnvalue_4 (Transformation|GetWorldLocation _grippable_magazine_mesh))
  (bind _returnvalue_5 (Math|Interpolation|VInterpTo _returnvalue_4 _returnvalue_2 _returnvalue_3 1.0))
  (Transformation|SetRelativeLocation (Variables|/Script/Engine.Actor|GetRootComponent _magazine) _returnvalue_5 false false)
  (return (Utilities|Operators|EqualEqual _returnvalue_2 _returnvalue_5 0.01)))

(fn LineTracefromBarrel
  (params (Start :type Vector) (End :type Vector))
  (bind _outhit (Collision|LineTraceByChannel Start End "TraceTypeQuery1" false 0 "None"))
  (return _outhit))

(fn GunLocationandDirection
  (params (Distance :type Float%20%28double-precision%29))
  (bind _gunmesh (Variables|Default|GetGunMesh))
  (bind _silenserattached (Variables|Default|GetSilenserAttached))
  (bind _returnvalue (Transformation|GetSocketLocation _gunmesh "Barrel"))
  (bind _returnvalue_2 (Transformation|GetSocketLocation _gunmesh "SilenserBarrel"))
  (bind _returnvalue_3 (Math|Vector|SelectVector _returnvalue_2 _returnvalue _silenserattached))
  (return (+ _returnvalue_3 (* (Math|Vector|GetForwardVector (Transformation|GetSocketRotation _gunmesh "Barrel")) Distance)) _returnvalue_3))

(fn ImpactDecals
  (params (Hit :type Hit%20Result%20Structure))
  (bind (_bblockinghit _binitialoverlap _time _distance _location _impactpoint _normal _impactnormal _physmat _hitactor _hitcomponent) (Collision|BreakHitResult Hit))
  (switch Utilities|FlowControl|Switch|SwitchonEPhysicalSurface (Variables|/Script/PhysicsCore.PhysicalMaterial|GetSurfaceType _physmat)
    (:SurfaceType_Default
      (CallFunction|BulletDefaultHitDecal _hitcomponent _impactpoint _normal))))

(fn BulletDefaultHitDecal
  (params (Hit%20Component :type Primitive%20Component%20Object%20Reference) (Get%20Location :type Vector) (Normal :type Vector))
  (bind _returnvalue (Class|GameplayStatics|SpawnDecalAttached "/Game/MilitarySimulator/JSG/Assets/Gun/MT_BulletHole.MT_BulletHole" "2.000000,2.000000,2.000000" Hit%20Component "None" Get%20Location (Math|Conversions|RotationFromXVector Normal) "KeepRelativeOffset" 0.0))
  (Utilities|IsValid _returnvalue
    (:Is%20Valid
      (Rendering|Components|Decal|SetFadeScreenSize _returnvalue 0.001))))

(fn RandomizeRecoil
  ;[1 1 1] Extreme Values If Gun Is Only Grabbed By Once
  (Variables|Default|SetRandomRecoilY (Math|Random|RandomFloatinRange -0.25 0.25))
  (Variables|Default|SetRandomRecoilZ (Math|Random|RandomFloatinRange 0.0 0.25)))

(fn RandomDamageSeed
  (return (Math|Random|RandomIntegerinRange 0 100)))

(fn ImpactSoundandParticles
  (params (Hit :type Hit%20Result%20Structure))
  (bind (_bblockinghit _binitialoverlap _time _distance _location _impactpoint _normal _impactnormal _physmat) (Collision|BreakHitResult Hit))
  (bind _surfacetype (Variables|/Script/PhysicsCore.PhysicalMaterial|GetSurfaceType _physmat))
  (if _bblockinghit
    (Niagara|SpawnSystematLocation (Utilities|Select :Index _surfacetype :SurfaceType_Default "/Niagara/DefaultAssets/Templates/Systems/SimpleExplosion.SimpleExplosion") _impactpoint (Math|Conversions|RotationFromXVector _impactnormal))
    (Audio|SpawnSoundatLocation (Utilities|Select :Index _surfacetype :SurfaceType_Default "/Game/MilitarySimulator/HSB/Assets/Sound/Rifle_Cue.Rifle_Cue") _impactpoint "0, 0, 0" 1.0 1.0 0.0 0 0)))

(fn ShowSlideGrip
  (Rendering|SetVisibility (Variables|Default|GetSlideMotionControllerHandMesh) false false)
  (if (Utilities|Enum|Equal(Enum) (Default|GetHeldbyHand (Variables|Default|GetCurlGrabComponentSlide)) "Left")
    (Rendering|SetVisibility (Variables|Default|GetSlideHand_L) true false)
    (else
      (Rendering|SetVisibility (Variables|Default|GetSlideHand_R) true false))))

(fn MappingContextGun
  (bind _grabcomponentsnap (Variables|Default|GetGrabComponentSnap))
  (bind _returnvalue (Default|GetHeldbyHand _grabcomponentsnap))
  (bind _returnvalue_2 (Utilities|Enum|Equal(Enum) _returnvalue "Left"))
  (bind _returnvalue_3 (select _returnvalue_2 "/Game/MilitarySimulator/HSB/Input/IMC_Weapon_Left.IMC_Weapon_Left" "/Game/MilitarySimulator/HSB/Input/IMC_Weapon_Right.IMC_Weapon_Right"))
  (Development|PrintString "JSG MappintContextGun")
  (bind _ascharacter (Utilities|Casting|CastToCharacter (Components|GetOwner)))
  (bind _asplayer_controller (Utilities|Casting|CastToPlayerController (Pawn|GetController _ascharacter)))
  (Input|EnableInput _asplayer_controller)
  (bind _ascharacter_2 (Utilities|Casting|CastToCharacter (Components|GetOwner)))
  (bind _asplayer_controller_2 (Utilities|Casting|CastToPlayerController (Pawn|GetController _ascharacter_2)))
  (Input|AddMappingContext (PlayerController|LocalPlayerSubsystems|GetEnhancedInputLocalPlayerSubsystem _asplayer_controller_2) _returnvalue_3 4 (LocalVariables|GetMappingOption))
  (Development|PrintString (Utilities|String|ToString(Text) (Utilities|Text|FormatText "JSG Mapping End, {IMC}" _returnvalue_3))))