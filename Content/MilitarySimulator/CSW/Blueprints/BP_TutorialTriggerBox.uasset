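; Tutorial trigger box that shows a widget component while something overlaps its box and hides it afterwards.
; The widget starts hidden at BeginPlay, and the Box begin and end overlap events toggle its visibility without filtering the overlapping actor.
; Every tick it yaws the widget toward the player pawn, ignoring height difference.
; A timeline that scales the widget and then hides it is present but never runs.
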(event OnComponentBeginOverlap(Box)
  (params (OverlappedComponent :type Primitive%20Component%20Object%20Reference) (OtherActor :type Actor%20Object%20Reference) (OtherComp :type Primitive%20Component%20Object%20Reference) (OtherBodyIndex :type Integer) (bFromSweep :type Boolean) (SweepResult :type Hit%20Result%20Structure%20%28by%20ref%29))
  (Rendering|SetVisibility (Variables|Default|GetWidget) true false))

(event OnComponentEndOverlap(Box)
  (params (OverlappedComponent :type Primitive%20Component%20Object%20Reference) (OtherActor :type Actor%20Object%20Reference) (OtherComp :type Primitive%20Component%20Object%20Reference) (OtherBodyIndex :type Integer))
  (Rendering|SetVisibility (Variables|Default|GetWidget) false false))

(event EventBeginPlay
  (Rendering|SetVisibility (Variables|Default|GetWidget) false false))

(event Collision|EventActorBeginOverlap
  (params (OtherActor :type Actor%20Object%20Reference)))

(event EventTick
  (params (DeltaSeconds :type Float%20%28single-precision%29))
  (bind _returnvalue (Game|Player|GetPlayerPawn 0))
  (bind _widget (Variables|Default|GetWidget))
  (bind _returnvalue_2 (Transformation|GetActorLocation _returnvalue))
  (bind _returnvalue_3 (Transformation|GetWorldLocation _widget))
  (bind _returnvalue_4 (- _returnvalue_2 _returnvalue_3))
  (Transformation|SetWorldRotation (Variables|Default|GetWidget) (Math|Conversions|RotationFromXVector (Math|Vector|MakeVector (.x _returnvalue_4) (.y _returnvalue_4) 0.0)) false false))

(fn ConstructionScript)