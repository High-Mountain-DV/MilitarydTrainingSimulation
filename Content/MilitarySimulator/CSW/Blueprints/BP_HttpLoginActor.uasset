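; BP_HttpLoginActor is a login-gated sliding door with a widget component, presumably the login prompt.
; BeginPlay treats a non-empty CSWGameInstance nickname as logged in, then opens the door and hides the widget.
; While that Login flag is set, box overlaps open and close the door without filtering the overlapping actor.
; A Timeline played forward or reversed slides the static mesh along its relative Y axis.
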(event OnComponentBeginOverlap(Box)
  (params (OverlappedComponent :type Primitive%20Component%20Object%20Reference) (OtherActor :type Actor%20Object%20Reference) (OtherComp :type Primitive%20Component%20Object%20Reference) (OtherBodyIndex :type Integer) (bFromSweep :type Boolean) (SweepResult :type Hit%20Result%20Structure%20%28by%20ref%29))
  (if (Variables|Default|GetbLogin)
    (CallFunction|OverlapOpen)
    (Rendering|SetVisibility (Variables|Default|GetWidgetComp) false false)))

(event OnComponentEndOverlap(Box)
  (params (OverlappedComponent :type Primitive%20Component%20Object%20Reference) (OtherActor :type Actor%20Object%20Reference) (OtherComp :type Primitive%20Component%20Object%20Reference) (OtherBodyIndex :type Integer))
  (if (Variables|Default|GetbLogin)
    (CallFunction|Close)))

(event Custom|close
  (bind _newtrack_0 (Timeline|Timeline Reverse)
    (:Update
      (Transformation|SetRelativeLocation (Variables|Default|GetStaticMesh) (Math|Vector|MakeVector 0.0 (Math|Float|Lerp 0.0 1e+02 _newtrack_0) 0.0) false false))))

(event Custom|OverlapOpen
  (bind _newtrack_0 (Timeline|Timeline Play)
    (:Update
      (Transformation|SetRelativeLocation (Variables|Default|GetStaticMesh) (Math|Vector|MakeVector 0.0 (Math|Float|Lerp 0.0 1e+02 _newtrack_0) 0.0) false false))))

(event EventBeginPlay
  (bind _ascswgame_instance (Utilities|Casting|CastToCSWGameInstance (Game|GetGameInstance)))
  (bind _output_get (Variables|Default|SetbLogin (not (Utilities|Array|IsEmpty (Class|CSWGameInstance|GetNickname _ascswgame_instance)))))
  (if _output_get
    (CallFunction|OverlapOpen)
    (Rendering|SetVisibility (Variables|Default|GetWidgetComp) false false)))

(event Collision|EventActorBeginOverlap
  (params (OtherActor :type Actor%20Object%20Reference)))

(event EventTick
  (params (DeltaSeconds :type Float%20%28single-precision%29)))

(event EventOpen
  (bind _newtrack_0 (Timeline|Timeline Play)
    (:Update
      (Transformation|SetRelativeLocation (Variables|Default|GetStaticMesh) (Math|Vector|MakeVector 0.0 (Math|Float|Lerp 0.0 1e+02 _newtrack_0) 0.0) false false))))

(fn ConstructionScript)