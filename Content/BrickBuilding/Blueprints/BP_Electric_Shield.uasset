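; Interactive electrical breaker box whose switch the player flips with E.
; Overlapping the Trigger enables input and shows a "Press E" prompt; leaving it disables input.
; Each press toggles TurnedOff, plays the breaker sound and runs a timeline forward or in reverse to rotate the Switch around its roll axis.
; The toggle drives only the sound and switch animation here, with no power logic.
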(event OnComponentBeginOverlap(Trigger)
  (params (OverlappedComponent :type Primitive%20Component%20Object%20Reference) (OtherActor :type Actor%20Object%20Reference) (OtherComp :type Primitive%20Component%20Object%20Reference) (OtherBodyIndex :type Integer) (bFromSweep :type Boolean) (SweepResult :type Hit%20Result%20Structure%20%28by%20ref%29))
  (Input|EnableInput (Game|GetPlayerController 0))
  (Development|PrintText "Press E" true false "(R=1.000000,G=1.000000,B=1.000000,A=1.000000)" 5.0))

(event OnComponentEndOverlap(Trigger)
  (params (OverlappedComponent :type Primitive%20Component%20Object%20Reference) (OtherActor :type Actor%20Object%20Reference) (OtherComp :type Primitive%20Component%20Object%20Reference) (OtherBodyIndex :type Integer))
  (Input|DisableInput (Game|GetPlayerController 0)))

(event EventBeginPlay)

(event Collision|EventActorBeginOverlap
  (params (OtherActor :type Actor%20Object%20Reference)))

(event EventTick
  (params (DeltaSeconds :type Float%20%28single-precision%29)))

(event Input|KeyboardEvents|E
  (params (Key :type Key%20Structure))
  (:Pressed
    (bind _output_get (Variables|Default|SetTurned%20off (not (Variables|Default|GetTurned%20off))))
    (if _output_get
      (Audio|SpawnSound2D "/Game/BrickBuilding/Sounds/A_Breaker_Sound_Cue.A_Breaker_Sound_Cue" 1.0 1.0 0.0 0)
      (bind _newtrack_0 (Timeline|Timeline_1 Play)
        (:Update
          (Transformation|SetRelativeRotation (Variables|Default|GetSwitch) (Math|Rotator|MakeRotator _newtrack_0 0.0 0.0) false false)))
      (else
        (Audio|SpawnSound2D "/Game/BrickBuilding/Sounds/A_Breaker_Sound_Cue.A_Breaker_Sound_Cue" 1.0 1.0 0.0 0)
        (Timeline|Timeline_1 Reverse)))))

(fn ConstructionScript)