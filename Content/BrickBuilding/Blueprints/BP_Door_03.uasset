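; BP_Door_03 is an interactive door that players swing open or shut with the E key.
; Entering its Trigger enables input, shows a prompt and makes the overlapping actor the door's owner; leaving reverses input and ownership.
; E calls a server RPC, which multicasts a toggle of IsClosed.
; The multicast plays a 2D sound and runs a Timeline forward or backward to drive Door01's relative yaw.
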(event OnComponentBeginOverlap(Trigger)
  (params (OverlappedComponent :type Primitive%20Component%20Object%20Reference) (OtherActor :type Actor%20Object%20Reference) (OtherComp :type Primitive%20Component%20Object%20Reference) (OtherBodyIndex :type Integer) (bFromSweep :type Boolean) (SweepResult :type Hit%20Result%20Structure%20%28by%20ref%29))
  (Input|EnableInput (Game|GetPlayerController 0))
  (Development|PrintText "Press E" true false "(R=1.000000,G=1.000000,B=1.000000,A=1.000000)" 5.0)
  (Actor|SetOwner OtherActor))

(event OnComponentEndOverlap(Trigger)
  (params (OverlappedComponent :type Primitive%20Component%20Object%20Reference) (OtherActor :type Actor%20Object%20Reference) (OtherComp :type Primitive%20Component%20Object%20Reference) (OtherBodyIndex :type Integer))
  (Input|DisableInput (Game|GetPlayerController 0))
  (Actor|SetOwner 0))

(event Custom|MulticastRPC_RotateDoor
  (bind _output_get (Variables|Default|SetIs%20Closed (not (Variables|Default|GetIs%20Closed))))
  (if _output_get
    (Audio|SpawnSound2D "/Game/BrickBuilding/Sounds/A_Open_Door_01_Cue.A_Open_Door_01_Cue" 1.0 1.0 0.0 0)
    (bind _newtrack_0 (Timeline|Timeline Play)
      (:Update
        (Transformation|SetRelativeRotation (Variables|Default|GetDoor01) (Math|Rotator|MakeRotator 0.0 0.0 _newtrack_0) false false)
        (Development|PrintString "Hello")))
    (else
      (Audio|SpawnSound2D "/Game/BrickBuilding/Sounds/A_Closing_Door_01_Cue.A_Closing_Door_01_Cue" 1.0 1.0 0.0 0)
      (Timeline|Timeline Reverse))))

(event Custom|ServerRPC_RotateDoor
  (CallFunction|MulticastRPCRotateDoor))

(event EventBeginPlay)

(event Collision|EventActorBeginOverlap
  (params (OtherActor :type Actor%20Object%20Reference)))

(event EventTick
  (params (DeltaSeconds :type Float%20%28single-precision%29)))

(event Input|KeyboardEvents|E
  (params (Key :type Key%20Structure :default "None"))
  (:Pressed
    (CallFunction|ServerRPCRotateDoor)
    (Development|PrintString "Prev ServerRPC")))

(fn ConstructionScript)